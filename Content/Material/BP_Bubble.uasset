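; BP_Bubble is a clickable floating bubble target that awards a point when popped.
; On BeginPlay it enables mouse click events and picks a randomized, upward-biased direction, then drifts along it at constant speed each Tick without sweeping.
; Clicking its Sphere while the first-person game mode is not game over increments the timer widget's score, spawns an explosion particle and pop sound, then destroys the bubble.
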(event `self.ReceiveBeginPlay`
  (bind _returnvalue (`GameplayStatics.GetPlayerController` 0))
  (`self.EnableInput` _returnvalue)
  (set `PlayerController.bEnableClickEvents` true _returnvalue)
  (set `self.MovementDirection` (`KismetMathLibrary.Normal` (`KismetMathLibrary.MakeVector` (`KismetMathLibrary.RandomFloatInRange` -1.0 1.0) (`KismetMathLibrary.RandomFloatInRange` -1.0 1.0) 2.0))))

(event `self.ReceiveTick`
  (params (DeltaSeconds :type "Float (single-precision)"))
  (`self.K2_AddActorWorldOffset` (* (* (`self.MovementDirection`) 80.0) DeltaSeconds)))

(event `self.Sphere.OnClicked`
  (params (TouchedComponent :type "PrimitiveComponent Object Reference") (ButtonPressed :type "Key Structure"))
  (bind _returnvalue (`SceneComponent.K2_GetComponentLocation` TouchedComponent))
  (bind _asbp_first_person_game_mode (cast `/Game/FirstPerson/Blueprints/BP_FirstPersonGameMode` (`GameplayStatics.GetGameMode`)))
  (if (not (`/Game/FirstPerson/Blueprints/BP_FirstPersonGameMode.IsGameOver` _asbp_first_person_game_mode))
    (bind _timerwidgetref (`/Game/FirstPerson/Blueprints/BP_FirstPersonGameMode.TimerWidgetRef` _asbp_first_person_game_mode))
    (set `/Game/Material/Timer.Score` (+ (`/Game/Material/Timer.Score` _timerwidgetref) 1) _timerwidgetref)
    (`GameplayStatics.SpawnEmitterAtLocation` "/Game/StarterContent/Particles/P_Explosion.P_Explosion" _returnvalue (struct) (1.0 1.0 1.0) true "AutoRelease")
    (`GameplayStatics.PlaySoundAtLocation` "/Game/Material/245645__unfa__cartoon-pop-clean.245645__unfa__cartoon-pop-clean" _returnvalue (struct) 1.0 1.0 0.0 null null null null)
    (`self.K2_DestroyActor`)))

(fn `UserConstructionScript`)